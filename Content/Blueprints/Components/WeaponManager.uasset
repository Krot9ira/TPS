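; Character component that manages two test weapons and switches between them on input.
; On BeginPlay a locally controlled character creates the ammo widget; otherwise the server spawns both weapons, attached hidden to a hand socket via multicast.
; Equip inputs go through server events to a multicast that swaps visibility, replaces the GAS fire ability with the weapon's own and rebinds ammo updates to the widget.
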(event `Multicast_Equip`
  (params (NewWeapon :type "/Game/Blueprints/Weapons/BP_BaseWeapon Object Reference"))
  (bind _currentweapon (`self.CurrentWeapon`))
  ;[1 1 1] Equip TODO Move it to GAS Ability (too lazy for now to do it)
  (`/Engine/EditorBlueprintResources/StandardMacros.IsValid` _currentweapon
    (:`Is Valid`
      (clear `/Game/Blueprints/Weapons/BP_BaseWeapon.AmmoChanged` _currentweapon)
      (`Actor.SetActorHiddenInGame` (`self.CurrentWeapon`) true)
      (`AbilitySystemComponent.ClearAbility` (`AbilitySystemBlueprintLibrary.GetAbilitySystemComponent` (`self.Character`)) (`self.CurrentFireAbility`)))
    (:`Is Not Valid`
      _))
  (bind _output_get (set `self.CurrentWeapon` NewWeapon))
  (bind _returnvalue (`KismetSystemLibrary.LoadClassAsset_Blocking` (`/Game/Blueprints/Weapons/BP_BaseWeapon.FireAbility` _output_get)))
  (bind _asgameplay_ability (castclass `GameplayAbility` _returnvalue)
    (:`then`
      (bind _returnvalue_2 (`AbilitySystemComponent.K2_GiveAbility` (`AbilitySystemBlueprintLibrary.GetAbilitySystemComponent` (`self.Character`)) _asgameplay_ability 1 3))
      (set `self.CurrentFireAbility` _returnvalue_2))
    (:`CastFailed`
      _))
  (`Actor.SetActorHiddenInGame` _output_get false)
  (`/Engine/EditorBlueprintResources/StandardMacros.IsValid` (`self.Ammo_W`)
    (:`Is Valid`
      (add `/Game/Blueprints/Weapons/BP_BaseWeapon.AmmoChanged` _output_get (delegate `UpdateAmmo`))
      (`/Game/Blueprints/Widgets/UW_Ammo.SetAmmo` (`self.Ammo_W`) (`/Game/Blueprints/Weapons/BP_BaseWeapon.Ammo` _output_get)))))

(event `EnhancedInput|/Game/Input/Actions/IA_EquipFirst`
  (params (ActionValue :type Boolean) (ElapsedSeconds :type "Float (double-precision)") (TriggeredSeconds :type "Float (double-precision)") (InputAction :type "InputAction Object Reference" :default "/Game/Input/Actions/IA_EquipFirst.IA_EquipFirst"))
  (:`Triggered`
    (`self.Server_EquipFirst`)))

(event `UpdateAmmo`
  (params (NewAmmoValue :type Integer))
  (`/Game/Blueprints/Widgets/UW_Ammo.SetAmmo` (`self.Ammo_W`) NewAmmoValue))

(event `Server_EquipFirst`
  ;[1 1 1] Equip TODO Move it to GAS Ability (too lazy for now to do it)
  (`self.Multicast_Equip` (`self.FirstWeapon`)))

(event `EnhancedInput|/Game/Input/Actions/IA_EquipSecond`
  (params (ActionValue :type Boolean) (ElapsedSeconds :type "Float (double-precision)") (TriggeredSeconds :type "Float (double-precision)") (InputAction :type "InputAction Object Reference" :default "/Game/Input/Actions/IA_EquipSecond.IA_EquipSecond"))
  (:`Triggered`
    (`self.Server_EquipSecond`)))

(event `Server_EquipSecond`
  ;[1 1 1] Equip TODO Move it to GAS Ability (too lazy for now to do it)
  (`self.Multicast_Equip` (`self.SecondWeapon`)))

(event `self.ReceiveBeginPlay`
  (bind _asbp_third_person_character (cast `/Game/Blueprints/Characters/BP_ThirdPersonCharacter` (`self.GetOwner`)))
  (bind _output_get (set `self.Character` _asbp_third_person_character))
  (if (`Pawn.IsLocallyControlled` _output_get)
    (bind _returnvalue (`|CreateWidget` "/Game/Blueprints/Widgets/UW_Ammo.UW_Ammo_C"))
    (bind _output_get_2 (set `self.Ammo_W` _returnvalue))
    (`UserWidget.AddToViewport` _output_get_2 0)
    (else
      ;[1 1 1] While no inventory and pickup system is meant to be just a spawning weapon here. -_-
      (if (`KismetSystemLibrary.IsServer`)
        (bind _returnvalue_2 (`|SpawnActorFromClass` "/Game/Blueprints/Weapons/BP_WeaponForTest1.BP_WeaponForTest1_C" (`KismetMathLibrary.MakeTransform` (0.0 0.0 0.0)) "Undefined" "MultiplyWithRoot" null null))
        (bind _output_get_3 (set `self.FirstWeapon` _returnvalue_2))
        (`self.Multicast_AttachToHandr` _output_get_3)
        (bind _returnvalue_3 (`|SpawnActorFromClass` "/Game/Blueprints/Weapons/BP_WeaponForTest2.BP_WeaponForTest2_C" (`KismetMathLibrary.MakeTransform` (0.0 0.0 0.0)) "Undefined" "MultiplyWithRoot" null null))
        (bind _output_get_4 (set `self.SecondWeapon` _returnvalue_3))
        (`self.Multicast_AttachToHandr` _output_get_4)))))

(event `Multicast_AttachToHandr`
  (params (Actor :type "Actor Object Reference"))
  (`Actor.K2_AttachToComponent` Actor (`Character.Mesh` (`self.Character`)) (`self.WeaponAttachSocketr`) "SnapToTarget" "SnapToTarget" "SnapToTarget" true)
  (`Actor.SetActorHiddenInGame` Actor true))