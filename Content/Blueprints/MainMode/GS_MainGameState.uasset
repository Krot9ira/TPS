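; Game state for the main mode that keeps the round's countdown clock, starting a five-minute round on BeginPlay.
; On the server, it sets TimeLeft and runs a looping one-second timer that decrements it, with no stop at zero in this graph.
; TimeLeft replicates with a RepNotify that fires the TimeLeftChanged dispatcher so listeners can react to each change.
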(event `SetRoundTimeAndStartCountDown`
  (params (TimeLeft :type "Float (double-precision)"))
  (if (`KismetSystemLibrary.IsServer`)
    (set `self.TimeLeft` TimeLeft)
    (bind _returnvalue (`KismetSystemLibrary.K2_SetTimerDelegate` (delegate `Deacrese`) 1.0 true true))
    (set `self.DeacreaseLeftTime` _returnvalue)))

(event `self.ReceiveBeginPlay`
  (`parent.ReceiveBeginPlay`)
  (`self.SetRoundTimeAndStartCountDown` 300.0))

(event `Deacrese`
  (`/Engine/EditorBlueprintResources/StandardMacros.DecrementFloat` (`self.TimeLeft`)))

(fn `OnRep_TimeLeft`
  (`self.TimeLeftChanged` (`self.TimeLeft`)))

(fn `UserConstructionScript`)