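; Base gameplay ability for weapon fire that loops a hip or aim-down-sight montage until input is released or ammo runs out.
; Each loop decrements the current WeaponManager weapon's ammo directly rather than through an ability cost, flagged as a stopgap.
; Fire notify events run an instant line trace from the player viewpoint with debug drawing.
; On authority, hit targets with an ability system receive a SetByCaller damage effect carrying the hit result.
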(event `self.K2_ActivateAbility`
  (bind (_owneractor _avataractor _playercontroller) (break `GameplayAbilityActorInfo` (`self.GetActorInfo`)))
  (bind (_location _rotation) (`Controller.GetPlayerViewPoint` _playercontroller))
  (set `self.StopFire` false)
  (bind _output_get (set `self.WeaponManager` (`Actor.GetComponentByClass` (`.AvatarActor` (break `GameplayAbilityActorInfo` (`self.GetActorInfo`))) "/Game/Blueprints/Components/WeaponManager.WeaponManager_C")))
  (`/Engine/EditorBlueprintResources/StandardMacros.IsValid` _output_get
    (:`Is Valid`
      (`|ExecutionSequence`
        (:`then_0`
          (bind _asynctaskproxy (`AbilityTask_WaitGameplayEvent.WaitGameplayEvent` (struct :`TagName` "Notify.Event.Fire") null)
            (:`then`
              (set `self.WaitFire` _asynctaskproxy)
              (bind _asynctaskproxy_2 (`AbilityTask_WaitInputRelease.WaitInputRelease` true)
                (:`then`
                  (set `self.WaitRealesed` _asynctaskproxy_2))
                (:`OnRelease`
                  (set `self.StopFire` true))))
            (:`EventReceived`
              ;[1 1 1] TODO For future is better to write custom abilitytargetdata and wait node because this node is destroy and spawn again and again abilitytargetdata actor and this is not good
              (bind (_asynctaskproxy_3 _data) (`AbilityTask_WaitTargetData.WaitTargetData` "WaitWanted" "Instant" "/Script/GameplayAbilities.GameplayAbilityTargetActor_SingleLineTrace" 999999.0 (struct :`Name` "BlockAll") true (make `GameplayAbilityTargetingLocationInfo` "LiteralTransform" (`KismetMathLibrary.MakeTransform` _location _rotation) _avataractor) (struct) null (struct) true)
                (:`ValidData`
                  (bind _returnvalue (`AbilitySystemBlueprintLibrary.GetHitResultFromTargetData` _data))
                  (`KismetSystemLibrary.DrawDebugBox` (`.Location` (`GameplayStatics.BreakHitResult` _returnvalue)) (3.0 3.0 3.0) (struct :`R` 0.081677 :`B` 1.0 :`A` 1.0) (struct) 1.0 5.0)
                  (`self.K2_HasAuthority`
                    (:`True`
                      (bind _returnvalue_2 (`AbilitySystemBlueprintLibrary.GetAbilitySystemComponent` (`.HitActor` (`GameplayStatics.BreakHitResult` _returnvalue))))
                      (`/Engine/EditorBlueprintResources/StandardMacros.IsValid` _returnvalue_2
                        (:`Is Valid`
                          (bind _returnvalue_3 (`AbilitySystemBlueprintLibrary.AssignTagSetByCallerMagnitude` (`AbilitySystemComponent.MakeOutgoingSpec` :`self` _returnvalue_2 :`GameplayEffectClass` (`self.DamageGameplayEffectClass`) :`Level` 1.0) (struct :`TagName` "Data.Damage") (`self.Damage`)))
                          (bind _returnvalue_4 (`AbilitySystemBlueprintLibrary.GetEffectContext` _returnvalue_3))
                          (`AbilitySystemBlueprintLibrary.EffectContextAddHitResult` _returnvalue_4 _returnvalue)
                          (`AbilitySystemComponent.BP_ApplyGameplayEffectSpecToTarget` (`self.GetAbilitySystemComponentFromActorInfo`) _returnvalue_3 _returnvalue_2))))))
                (:`Cancelled`)))))
        (:`then_1`
          ;[1 1 1] !!! Its not a good way| In good way i need to override some function in Gameplay ability to check apply cost and disable replication of ammo while shooting
          (bind _canshoot (`/Game/Blueprints/Weapons/BP_BaseWeapon.DeacreseAmmoCanShoot` (`/Game/Blueprints/Components/WeaponManager.CurrentWeapon` (`self.WeaponManager`)) :!label _label))
          (if _canshoot
            (`AbilityTask_PlayMontageAndWait.CreatePlayMontageAndWaitProxy` "None" (select `bool` (`GameplayTagAssetInterface.HasMatchingGameplayTag` (`self.GetAbilitySystemComponentFromActorInfo`) (struct :`TagName` "State.AimDownSight")) :`false` (`self.FireMontage`) :`true` (`self.FireAimMontage`)) 1.0 "None" false 1.0 0.0 true
              (:`OnCompleted`
                (if (`self.StopFire`)
                  (`self.K2_EndAbilityLocally`)
                  (else
                    (goto _label))))
              (:`OnInterrupted`
                (`self.K2_EndAbility` :!label _label_2))
              (:`OnCancelled`
                (goto _label_2)))
            (else
              (`self.K2_EndAbility`))))))
    (:`Is Not Valid`
      (`self.K2_EndAbility`))))

(event `self.K2_OnEndAbility`
  (params (bWasCancelled :type Boolean))
  (bind _waitrealesed (`self.WaitRealesed`))
  (bind _waitfire (`self.WaitFire`))
  (`/Engine/EditorBlueprintResources/StandardMacros.IsValid` _waitfire
    (:`Is Valid`
      (`GameplayTask.EndTask` _waitfire))
    (:`Is Not Valid`
      _))
  (`/Engine/EditorBlueprintResources/StandardMacros.IsValid` _waitrealesed
    (:`Is Valid`
      (`GameplayTask.EndTask` _waitrealesed))
    (:`Is Not Valid`
      _))
  (set `self.WeaponManager` null))